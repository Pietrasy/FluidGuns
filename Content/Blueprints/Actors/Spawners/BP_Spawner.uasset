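; BP_Spawner is a world pickup that shows an item's mesh and gives that item to the player on touch.
; On BeginPlay it async-loads the item data asset, applies its static mesh and starts a timeline that animates the mesh's height.
; Sphere overlap with an actor tagged Character.Player executes the data asset's Action on that player, plays a pickup sound and destroys the spawner.
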(event OnComponentBeginOverlap(SphereCollision)
  (params (OverlappedComponent :type Primitive%20Component%20Object%20Reference) (OtherActor :type Actor%20Object%20Reference) (OtherComp :type Primitive%20Component%20Object%20Reference) (OtherBodyIndex :type Integer) (bFromSweep :type Boolean) (SweepResult :type Hit%20Result%20Structure%20%28by%20ref%29))
  ;[1 1 1] Detect collision with player
  (bind _gameplaytagcontainer (Class|BPIGameplayTag|RetrieveGameplayTagContainer(Message) OtherActor))
  (if (GameplayTags|HasTag _gameplaytagcontainer "(TagName=\"Character.Player\")")
    (bind _asbp_player (Utilities|Casting|CastToBP_Player OtherActor))
    (CallFunction|PickUp _asbp_player)
    (Actor|DestroyActor)))

(event Custom|MeshMovement
  (bind _itemstaticmesh (Variables|Default|GetItemStaticMesh))
  (bind _relativelocation (Variables|/Script/Engine.SceneComponent|GetRelativeLocation _itemstaticmesh))
  ;[1 1 1] Mesh movement
  (bind _interpolation (Timeline|MeshMovement_Timeline PlayFromStart)
    (:Update
      (Transformation|SetRelativeLocation (Variables|Default|GetItemStaticMesh) (Math|Vector|MakeVector (.x _relativelocation) (.y _relativelocation) _interpolation) false false))))

(event EventBeginPlay
  (|CallParentFunction)
  ;[1 1 1] Load item data asset and set spawner static mesh
  (bind _object (Utilities|AsyncLoadAsset (Variables|Default|GetItemToSpawn))
    (:Completed
      (bind _asfg_pda_item (Utilities|Casting|CastToFG_PDA_Item _object))
      (Variables|Default|SetItemDA _asfg_pda_item)
      (CallFunction|SetSpawnerStaticMesh)
      (CallFunction|MeshMovement))))

(fn ConstructionScript)

(fn SetSpawnerStaticMesh
  (Components|StaticMesh|SetStaticMesh (Variables|Default|GetItemStaticMesh) (Variables|/Script/FluidGuns.FG_PDA_Item|GetItemStaticMesh (Variables|Default|GetItemDA)))
  (return))

(fn PickUp
  (params (Player :type FG%20Player%20Object%20Reference))
  (bind _itemda (Variables|Default|GetItemDA)
    (:then
      (Class|FGAction|Execute (Variables|/Script/FluidGuns.FG_PDA_Item|GetAction (Variables|Default|GetItemDA)) _itemda Player)
      (CallFunction|PlayPickupSound)
      (return))
    (:else)))

(fn PlayPickupSound
  (Audio|PlaySoundatLocation (Variables|Default|GetPickupSound) (Transformation|GetActorLocation) "0, 0, 0" 1.0 1.0 0.0 0 0 0 0)
  (return))