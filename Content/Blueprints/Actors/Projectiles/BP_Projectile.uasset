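; Fluid projectile actor that leaves a colored splash decal where it hits and then destroys itself.
; On BeginPlay it looks up its color from the FluidType gameplay tag and passes it to the mesh through custom primitive data.
; On collision it spawns a timed decal aligned to the impact normal with randomized rotation, tinting it through a dynamic material instance.
; The construction script applies InitialSpeed to the projectile component.
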(event OnComponentHit(SphereCollision)
  (params (HitComponent :type Primitive%20Component%20Object%20Reference) (OtherActor :type Actor%20Object%20Reference) (OtherComp :type Primitive%20Component%20Object%20Reference) (NormalImpulse :type Vector :default "0, 0, 0") (Hit :type Hit%20Result%20Structure%20%28by%20ref%29))
  (bind (_bblockinghit _binitialoverlap _time _distance _location _impactpoint _normal _impactnormal) (Collision|BreakHitResult Hit))
  ;[1 1 1] Spawn decal at hit moment
  (bind _newrotator (CallFunction|RandomDecalRotation _impactnormal))
  (bind _returnvalue (Rendering|Decal|SpawnDecalatLocation "/Game/Art/Materials/Decals/Splash/M_Splash.M_Splash" (Variables|Default|GetDecalSize) _location _newrotator (Variables|Default|GetDecalLifeSpan)))
  ;[1 1 1] Set decal color
  (bind _returnvalue_2 (Rendering|Material|CreateDynamicMaterialInstance _returnvalue :!class /Script/Engine.DecalComponent))
  (Rendering|Material|SetVectorParameterValue _returnvalue_2 "Color" (Variables|Default|GetFluidColor) :!class /Script/Engine.MaterialInstanceDynamic)
  (Actor|DestroyActor))

(event EventBeginPlay
  (|CallParentFunction)
  ;[1 1 1] Set projectile color
  (bind _fluidcolor (CallFunction|GetFluidColorbyGameplayTag (Variables|Default|GetFluidType)))
  (bind _output_get (Variables|Default|SetFluidColor _fluidcolor))
  (Rendering|Material|SetCustomPrimitiveDataVector4 (Variables|Default|GetProjectileStaticMesh) 0 (Math|Vector4|MakeVector4 (.R (Math|Color|BreakColor _output_get)) (.G (Math|Color|BreakColor _output_get)) (.B (Math|Color|BreakColor _output_get)) (.A (Math|Color|BreakColor _output_get)))))

(fn ConstructionScript
  (Variables|/Script/Engine.ProjectileMovementComponent|SetInitialSpeed (Variables|Default|GetProjectileComponent) (Variables|Default|GetInitialSpeed)))

(fn RandomDecalRotation
  (params (ImpactNormal :type Vector))
  (bind _returnvalue (Math|Conversions|RotationFromXVector ImpactNormal))
  (bind (_x _y _z) (Math|Rotator|BreakRotIntoAxes _returnvalue))
  (return (Math|Rotator|MakeRotationfromAxes _x _y (Math|Vector|RotateVectorAroundAxis _z (Math|Random|RandomFloatinRange 0.0 3.6e+02) _x))))