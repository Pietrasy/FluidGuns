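; BP_FluidGun is a fluid gun that pumps up pressure through an addon and fires projectiles.
; Pump has the pump addon compute the new pressure, then plays a timeline that slides it along X.
; Fire is blocked while pumping; if the parent Fire succeeds, it spawns BP_Projectile at the FireOffset socket using Range as speed and the tank's fluid tag.
; OnSetFluidGun stops the timeline and clears the pumping state.
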(event Custom|OnPump
  (params (Pump :type Static%20Mesh%20Component%20Object%20Reference))
  ;[1 1 1] Pump addon
  (bind _interpolation (Timeline|PumpMovement_Timeline PlayFromStart)
    (:Update
      (Transformation|SetRelativeLocation Pump (Math|Vector|MakeVector _interpolation 0.0 0.0) false false))
    (:Finished
      (Variables|Default|SetIsPumping false))))

(event Custom|OnSetFluidGun
  (Audio|Components|Audio|Stop (Variables|Default|GetPumpMovement_Timeline))
  (Variables|Default|SetIsPumping false))

(event EventBeginPlay
  (|CallParentFunction)
  (EventDispatchers|BindEventtoOnSetGun (EventDispatchers|CreateEvent :!event Custom|OnSetFluidGun)))

(fn ConstructionScript)

(fn Pump
  (bind _fluidgunparameters (Variables|Default|GetFluidGunParameters))
  (bind (_pressure _maxpressure) (Utilities|Struct|BreakFluidGunParameters _fluidgunparameters))
  ;[1 1 1] Check if Pump timeline is already playing.
  (if (not (Audio|Components|Audio|IsPlaying (Variables|Default|GetPumpMovement_Timeline)))
    (Variables|Default|SetIsPumping true)
    ;[1 1 1] Get pump addon
    (bind _returnvalue (Class|FGFluidGun|GetAddon "(TagName=\"Addon.Pump\")"))
    (LocalVariables|SetPump _returnvalue)
    (LocalVariables|GetPump
      (:then
        ;[1 1 1] Change pressure level
        (bind _newpressure (Class|FGAddonInterface|ChangePressureLevel(Message) (LocalVariables|GetPump) _pressure _maxpressure))
        (|SetBy-RefVar (Utilities|Struct|BreakFluidGunParameters (Variables|Default|GetFluidGunParameters)) _newpressure)
        (CallFunction|OnPump (LocalVariables|GetPump))
        (return))
      (:else
        (return)))
    (else
      (return))))

(fn Fire
  (if (not (Variables|Default|GetIsPumping))
    (bind _bcanshot (|CallParentFunction))
    (if _bcanshot
      (Game|SpawnActorfromClass "/Game/Blueprints/Actors/Projectiles/BP_Projectile.BP_Projectile_C" (Transformation|GetSocketTransform (Variables|Default|GetFluidGunStaticMesh) "FireOffset" "RTS_World") "Undefined" "MultiplyWithRoot" 0 (Utilities|Struct|BreakFluidGunParameters (Variables|Default|GetFluidGunParameters)) (Utilities|Struct|BreakTankProperties (Variables|Default|GetTank)) 0)
      (return false))))