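; Interactable fluid source that refills the player's fluid gun tank with its fluid type, which also sets the mesh color and widget prompt.
; While a player-tagged actor overlaps the sphere, a looping timer compares camera facing against an angle threshold to show the prompt and enable interaction.
; On interact, it sends a refill message to the interactor's fluid gun component and plays a pouring or wrong sound based on the result.
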(event OnComponentBeginOverlap(SphereCollision)
  (params (OverlappedComponent :type Primitive%20Component%20Object%20Reference) (OtherActor :type Actor%20Object%20Reference) (OtherComp :type Primitive%20Component%20Object%20Reference) (OtherBodyIndex :type Integer) (bFromSweep :type Boolean) (SweepResult :type Hit%20Result%20Structure%20%28by%20ref%29))
  ;[1 1 1] When actor overlap with player, start timer.
  (Utilities|CheckifOverlappedActorIsPlayer OtherActor
    (:True
      (bind _returnvalue (Utilities|Time|SetTimerbyFunctionName 0 "CheckIfPlayerIsLooking" 0.1 true true))
      (Variables|Default|SetTimerHandle _returnvalue))))

(event OnComponentEndOverlap(SphereCollision)
  (params (OverlappedComponent :type Primitive%20Component%20Object%20Reference) (OtherActor :type Actor%20Object%20Reference) (OtherComp :type Primitive%20Component%20Object%20Reference) (OtherBodyIndex :type Integer))
  ;[1 1 1] On end overlap with player, collapse widget, set flag to false and clear timer.
  (Utilities|CheckifOverlappedActorIsPlayer OtherActor
    (:True
      (Widget|SetVisibility (Variables|Default|GetInteractionWidget) "Collapsed")
      (Variables|Default|SetIsInteractable false)
      (Utilities|Time|ClearandInvalidateTimerbyHandle (Variables|Default|GetTimerHandle)))))

(event EventInteractwith
  (params (Interactor :type Actor%20Object%20Reference))
  ;[1 1 1] Call RefillTank function to Interactor
  (if (Variables|Default|GetIsInteractable)
    (bind _fluidguncomponent (Class|BPIPlayer|ReturnFluidGunComponent(Message) Interactor))
    (Utilities|IsValid _fluidguncomponent
      (:Is%20Valid
        (bind _issuccess (Class|BPIFluidGunComponent|RefillTank(Message) _fluidguncomponent (Variables|Default|GetFluidSourceType)))
        (if _issuccess
          (CallFunction|PlayPouringSound)
          (else
            (CallFunction|PlayWrongSound)))))))

(event EventBeginPlay
  (|CallParentFunction)
  (CallFunction|CacheInteractionWidget) ; Cache Interface Widget reference to variable
  (Default|SetFluidSourcePrompt (Variables|Default|GetInteractionWidget) (Variables|Default|GetFluidSourceType)) ; Set appearance Interface Widget prompt
  (CallFunction|SetFluidColor (Variables|Default|GetFluidSourceType)) ; Set fluid material in actor
)

(fn ConstructionScript
  (|CallParentFunction))

(fn SetFluidColor
  (params (FluidTag :type Gameplay%20Tag%20Structure))
  (bind _fluidcolor (CallFunction|GetFluidColorbyGameplayTag FluidTag))
  (Rendering|Material|SetCustomPrimitiveDataVector4 (Variables|Default|GetFluidSourceStaticMesh) 0 (Math|Vector4|MakeVector4 (.r _fluidcolor) (.g _fluidcolor) (.b _fluidcolor) (.a _fluidcolor)))
  (return))

(fn CacheInteractionWidget
  (bind _aswbp_interaction_widget (Utilities|Casting|CastToWBP_InteractionWidget (UserInterface|GetWidget (Variables|Default|GetInteractionWidgetComponent))))
  (Variables|Default|SetInteractionWidget _aswbp_interaction_widget)
  (return))

(fn CheckifPlayerIsLooking
  (if (< (LocalVariables|GetAngle) (CallFunction|GetDotProduct)) ; If Angle is greater than dot product,\nshow interaction widget.
    (Widget|SetVisibility (Variables|Default|GetInteractionWidget) "Visible")
    (Variables|Default|SetIsInteractable true)
    (return)
    (else
      (Widget|SetVisibility (Variables|Default|GetInteractionWidget) "Collapsed")
      (Variables|Default|SetIsInteractable false)
      (return))))

(fn GetDotProduct
  (bind _returnvalue (Game|GetPlayerCameraManager 0))
  (return (Math|Vector|DotProduct (Transformation|GetActorForwardVector _returnvalue) (Math|Vector|GetUnitDirection(Vector) (Camera|GetCameraLocation _returnvalue) (Transformation|GetActorLocation)))))

(fn PlayPouringSound
  (Variables|Default|GetPouringSound_Instance
    (:then
      (Audio|Components|Audio|Stop (Variables|Default|GetPouringSound_Instance)))
    (:else
      _))
  (bind _returnvalue (Audio|SpawnSoundAttached (Variables|Default|GetPouringSound) (Variables|Default|GetFluidSourceStaticMesh) "None" "0, 0, 0" "0, 0, 0" "KeepRelativeOffset" false 1.0 1.0 0.0 0 0))
  (Variables|Default|SetPouringSound_Instance _returnvalue)
  (return))

(fn PlayWrongSound
  (Variables|Default|GetPouringSound_Instance
    (:then
      (Audio|Components|Audio|Stop (Variables|Default|GetPouringSound_Instance)))
    (:else
      _))
  (bind _returnvalue (Audio|SpawnSoundAttached "/Game/Art/SFX/A_Wrong.A_Wrong" (Variables|Default|GetFluidSourceStaticMesh) "None" "0, 0, 0" "0, 0, 0" "KeepRelativeOffset" false 1.0 1.0 0.0 0 0))
  (Variables|Default|SetPouringSound_Instance _returnvalue)
  (return))