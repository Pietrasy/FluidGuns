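; BP_WaterSource is an interactable fluid source actor that lets the player refill a tank with its FluidSourceType.
; On BeginPlay it sets the prompt on its interaction widget to match that type.
; Sphere overlaps show or hide the prompt and toggle interactability, identifying the player by the Character.Player gameplay tag instead of a cast.
; When interacted with while in range, it sends a refill message with the fluid type to the interactor.
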(event OnComponentBeginOverlap(SphereCollision)
  (params (OverlappedComponent :type Primitive%20Component%20Object%20Reference) (OtherActor :type Actor%20Object%20Reference) (OtherComp :type Primitive%20Component%20Object%20Reference) (OtherBodyIndex :type Integer) (bFromSweep :type Boolean) (SweepResult :type Hit%20Result%20Structure%20%28by%20ref%29))
  (Utilities|CheckifOverlappedActorIsPlayer OtherActor
    (:True
      (Widget|SetVisibility (Variables|Default|GetInteractionWidget) "Visible")
      (Variables|Default|SetIsInteractable true))))

(event OnComponentEndOverlap(SphereCollision)
  (params (OverlappedComponent :type Primitive%20Component%20Object%20Reference) (OtherActor :type Actor%20Object%20Reference) (OtherComp :type Primitive%20Component%20Object%20Reference) (OtherBodyIndex :type Integer))
  (Utilities|CheckifOverlappedActorIsPlayer OtherActor
    (:True
      (Widget|SetVisibility (Variables|Default|GetInteractionWidget) "Collapsed")
      (Variables|Default|SetIsInteractable false))))

(event EventInteractwith
  (params (Interactor :type Actor%20Object%20Reference))
  (if (Variables|Default|GetIsInteractable)
    (Class|BPIInteraction|RefillTank(Message) Interactor (Variables|Default|GetFluidSourceType))))

(event EventBeginPlay
  (bind _aswbp_interaction_widget (Utilities|Casting|CastToWBP_InteractionWidget (UserInterface|GetWidget (Variables|Default|GetInteractionWidgetComponent))))
  (Variables|Default|SetInteractionWidget _aswbp_interaction_widget)
  (Default|SetFluidSourcePrompt (Variables|Default|GetInteractionWidget) (Variables|Default|GetFluidSourceType)))

(fn ConstructionScript)