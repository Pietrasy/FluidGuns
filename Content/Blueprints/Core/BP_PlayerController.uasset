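; Player controller that handles first-person-style movement, smoothed look and interaction for BP_Player through Enhanced Input.
; On BeginPlay it caches the player character and adds the default mapping context.
; Move input drives the character along control-rotation right and capsule forward vectors, while look input is eased with FInterpTo before adding yaw and pitch.
; Interaction casts a visibility line trace from the camera and sends an interact message to the hit actor.
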(event EventBeginPlay
  (|CallParentFunction)
  (CallFunction|CachePlayerCharacter)
  (CallFunction|AddMappingContext))

(event Input|EnhancedActionEvents|EnhancedInputActionIA_Move
  (params (ActionValue :type Vector%202D%20Structure) (ElapsedSeconds :type Float%20%28double-precision%29) (TriggeredSeconds :type Float%20%28double-precision%29) (InputAction :type Input%20Action%20Object%20Reference :default "/Game/Inputs/Actions/IA_Move.IA_Move"))
  ;[1 1 1] Character movement
  (Pawn|Input|AddMovementInput (Variables|Default|GetPlayerCharacter) (Math|Vector|GetRightVector (Pawn|GetControlRotation :!class /Script/Engine.Controller)) (.x ActionValue) false)
  (Pawn|Input|AddMovementInput (Variables|Default|GetPlayerCharacter) (Math|Vector|GetForwardVector (Variables|/Script/Engine.Character|GetCapsuleComponent (Variables|Default|GetPlayerCharacter))) (.y ActionValue) false))

(event Input|EnhancedActionEvents|EnhancedInputActionIA_Look
  (params (ActionValue :type Vector%202D%20Structure) (ElapsedSeconds :type Float%20%28double-precision%29) (TriggeredSeconds :type Float%20%28double-precision%29) (InputAction :type Input%20Action%20Object%20Reference :default "/Game/Inputs/Actions/IA_Look.IA_Look"))
  ;[1 1 1] Camera movement
  (CallFunction|LookInterpolationRelativetoXAxis (.x ActionValue) 1.2e+02)
  (CallFunction|LookInterpolationRelativetoYAxis (.y ActionValue) 1.2e+02))

(event Input|EnhancedActionEvents|EnhancedInputActionIA_Interaction
  (params (ActionValue :type Boolean) (ElapsedSeconds :type Float%20%28double-precision%29) (TriggeredSeconds :type Float%20%28double-precision%29) (InputAction :type Input%20Action%20Object%20Reference :default "/Game/Inputs/Actions/IA_Interaction.IA_Interaction"))
  ;[1 1 1] Cast trace to try interact with something.
  (:Started
    (CallFunction|TryInteraction)))

(fn ConstructionScript)

(fn TryInteraction
  (bind (_start _end) (|Findstartandendoftracevector))
  (bind _outhit (Collision|LineTraceByChannel _start _end "TraceTypeQuery1" false 0 "None" true "(R=1.000000,G=0.000000,B=0.000000,A=1.000000)" "(R=0.000000,G=1.000000,B=0.000000,A=1.000000)" 15.0))
  (bind _output_get (LocalVariables|SetHitActor (.HitActor (Collision|BreakHitResult _outhit))))
  (Class|BPIInteraction|Interactwith(Message) _output_get (Variables|Default|GetPlayerCharacter))
  (return))

(fn AddMappingContext
  (Input|AddMappingContext (PlayerController|LocalPlayerSubsystems|GetEnhancedInputLocalPlayerSubsystem) "/Game/Inputs/IMC_Default.IMC_Default" 0 "(bIgnoreAllPressedKeysUntilRelease=True,bForceImmediately=False,bNotifyUserSettings=False)")
  (return))

(fn CachePlayerCharacter
  (bind _asbp_player (Utilities|Casting|CastToBP_Player (Game|GetPlayerCharacter 0)))
  (Variables|Default|SetPlayerCharacter _asbp_player)
  (return))

(fn LookInterpolationRelativetoXAxis
  (params (ValueX :type Float%20%28double-precision%29) (InterpSpeed :type Float%20%28double-precision%29))
  (bind _output_get (Variables|Default|SetInputAxisLookX (Math|Interpolation|FInterpTo (Variables|Default|GetInputAxisLookX) ValueX (Utilities|Time|GetWorldDeltaSeconds) 1.2e+02)))
  (Class|PlayerController|AddYawInput _output_get)
  (return))

(fn LookInterpolationRelativetoYAxis
  (params (ValueX :type Float%20%28double-precision%29) (InterpSpeed :type Float%20%28double-precision%29))
  (bind _output_get (Variables|Default|SetInputAxisLookY (Math|Interpolation|FInterpTo (Variables|Default|GetInputAxisLookY) ValueX (Utilities|Time|GetWorldDeltaSeconds) InterpSpeed)))
  (Class|PlayerController|AddPitchInput _output_get)
  (return))