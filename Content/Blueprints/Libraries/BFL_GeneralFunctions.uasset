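; Blueprint function library with lookups that translate a fluid gameplay tag into a color or a name.
; Both functions scan every row of DT_FluidColors and exact-match the row's FluidType against the given tag, returning that row's Color or its row name.
; With no match, they return the last value stored during the loop instead of a dedicated default.
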(fn GetFluidColorbyGameplayTag
  (params (FluidTag :type Gameplay%20Tag%20Structure))
  (bind _outrownames (DataTable|GetDataTableRowNames "/Game/Blueprints/Data/DataTables/DT_FluidColors.DT_FluidColors"))
  (for _array_element _outrownames
    (bind _returnvalue (Utilities|GetDataTableRow "/Game/Blueprints/Data/DataTables/DT_FluidColors.DT_FluidColors" _array_element)
      (:then
        (LocalVariables|SetColorFromDT (.Color (Utilities|Struct|BreakSFluidColors _returnvalue)))
        (if (GameplayTags|MatchesTag (.FluidType (Utilities|Struct|BreakSFluidColors _returnvalue)) FluidTag true)
          (return (LocalVariables|GetColorFromDT))))))
  (return (LocalVariables|GetColorFromDT)))

(fn GetFluidNamebyGameplayTag
  (params (FluidTag :type Gameplay%20Tag%20Structure))
  (bind _outrownames (DataTable|GetDataTableRowNames "/Game/Blueprints/Data/DataTables/DT_FluidColors.DT_FluidColors"))
  (for _array_element _outrownames
    (LocalVariables|SetName _array_element)
    (bind _returnvalue (Utilities|GetDataTableRow "/Game/Blueprints/Data/DataTables/DT_FluidColors.DT_FluidColors" (LocalVariables|GetName))
      (:then
        (if (GameplayTags|MatchesTag (Utilities|Struct|BreakSFluidColors _returnvalue) FluidTag true)
          (return (LocalVariables|GetName))))))
  (return (LocalVariables|GetName)))