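; Player component that handles fluid gun controls: firing, pumping, switching guns and opening the tank selection widget.
; It adds its own Enhanced Input mapping context and attaches each spawned gun to the character's GunSocket.
; Guns are drawn by gameplay tag, through slot keys or looping next/previous cycling over owned guns.
; Pumping broadcasts pressure and fluid amount for UI, while refills require an exact fluid tag match.
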(event Custom|Pump
  ;[1 1 1] Use fluid gun pump and update its parameters in widget.
  (Default|Pump (Variables|Default|GetFluidGun))
  (|CallOnGunParameters))

(event Custom|OnFluidGunSpawn
  ;[1 1 1] Attach fluid gun to player character when it is spawned.
  (bind _asbp_fluid_gun (Utilities|Casting|CastToBP_FluidGun (Variables|Default|GetCurrentGun)))
  (bind _output_get (Variables|Default|SetFluidGun _asbp_fluid_gun))
  (Transformation|AttachComponentToComponent _output_get (Variables|/Game/Blueprints/Characters/BP_Player.BP_Player_C|GetGunSocket (Variables|Default|GetPlayerCharacter)) "None" "SnapToTarget" "SnapToTarget" "SnapToTarget" true))

(event EventBeginPlay
  (|CallParentFunction)
  (EventDispatchers|BindEventtoOnSpawnFluidGun (EventDispatchers|CreateEvent :!event Custom|OnFluidGunSpawn))
  (CallFunction|SetMappingContext))

(event Input|EnhancedActionEvents|EnhancedInputActionIA_Fire
  (params (ActionValue :type Boolean) (ElapsedSeconds :type Float%20%28double-precision%29) (TriggeredSeconds :type Float%20%28double-precision%29) (InputAction :type Input%20Action%20Object%20Reference :default "/Game/Inputs/Actions/IA_Fire.IA_Fire"))
  (:Started
    (bind _currentgun (Variables|Default|GetCurrentGun)
      (:then
        (Class|FGFluidGun|Fire _currentgun))
      (:else))))

(event Input|EnhancedActionEvents|EnhancedInputActionIA_NextGun
  (params (ActionValue :type Boolean) (ElapsedSeconds :type Float%20%28double-precision%29) (TriggeredSeconds :type Float%20%28double-precision%29) (InputAction :type Input%20Action%20Object%20Reference :default "/Game/Inputs/Actions/IA_NextGun.IA_NextGun"))
  (:Started
    (bind _fluidguntag (CallFunction|NextFluidGun true))
    (if (GameplayTags|IsGameplayTagValid _fluidguntag)
      (Class|FGFluidGunComponent|DrawFluidGun _fluidguntag))))

(event Input|EnhancedActionEvents|EnhancedInputActionIA_PreviousGun
  (params (ActionValue :type Boolean) (ElapsedSeconds :type Float%20%28double-precision%29) (TriggeredSeconds :type Float%20%28double-precision%29) (InputAction :type Input%20Action%20Object%20Reference :default "/Game/Inputs/Actions/IA_PreviousGun.IA_PreviousGun"))
  (:Started
    (bind _fluidguntag (CallFunction|PreviousFluidGun true))
    (if (GameplayTags|IsGameplayTagValid _fluidguntag)
      (Class|FGFluidGunComponent|DrawFluidGun _fluidguntag))))

(event Input|EnhancedActionEvents|EnhancedInputActionIA_Pump
  (params (ActionValue :type Boolean) (ElapsedSeconds :type Float%20%28double-precision%29) (TriggeredSeconds :type Float%20%28double-precision%29) (InputAction :type Input%20Action%20Object%20Reference :default "/Game/Inputs/Actions/IA_Pump.IA_Pump"))
  (:Started
    (Variables|Default|GetCurrentGun
      (:then
        (CallFunction|Pump))
      (:else))))

(event Input|EnhancedActionEvents|EnhancedInputActionIA_ShowSelectTankWidget
  (params (ActionValue :type Boolean) (ElapsedSeconds :type Float%20%28double-precision%29) (TriggeredSeconds :type Float%20%28double-precision%29) (InputAction :type Input%20Action%20Object%20Reference :default "/Game/Inputs/Actions/IA_ShowSelectTankWidget.IA_ShowSelectTankWidget"))
  (:Started
    (Variables|Default|GetCurrentGun
      (:then
        (Default|CallShowSelectTankWidget))
      (:else))))

(event Input|EnhancedActionEvents|EnhancedInputActionIA_Slot1
  (params (ActionValue :type Boolean) (ElapsedSeconds :type Float%20%28double-precision%29) (TriggeredSeconds :type Float%20%28double-precision%29) (InputAction :type Input%20Action%20Object%20Reference :default "/Game/Inputs/Actions/IA_Slot1.IA_Slot1"))
  (Variables|Default|GetCurrentGun
    (:then
      (Class|FGFluidGunComponent|DrawFluidGun "(TagName=\"Gun.Pistol\")"))
    (:else)))

(event Input|EnhancedActionEvents|EnhancedInputActionIA_Slot2
  (params (ActionValue :type Boolean) (ElapsedSeconds :type Float%20%28double-precision%29) (TriggeredSeconds :type Float%20%28double-precision%29) (InputAction :type Input%20Action%20Object%20Reference :default "/Game/Inputs/Actions/IA_Slot2.IA_Slot2"))
  (Variables|Default|GetCurrentGun
    (:then
      (Class|FGFluidGunComponent|DrawFluidGun "(TagName=\"Gun.Rifle\")"))
    (:else)))

(fn NextFluidGun
  (params (EnableIndexLoop :type Boolean))
  (if (Utilities|Array|IsNotEmpty (Variables|Default|GetOwnedGuns)) ; Check if array is empty.
    ;[1 1 1] Cache current fluid gun index and check if it is a valid index in the OwnedGuns array.
    (bind _output_get (LocalVariables|SetCurrentIndex (Class|FGFluidGunComponent|GetCurrentFluidGunIndex)))
    (if (Utilities|Array|IsValidIndex (Variables|Default|GetOwnedGuns) _output_get)
      (LocalVariables|SetNextIndex (+ (LocalVariables|GetCurrentIndex) 1))
      (LocalVariables|SetCurrentIndex (Math|Integer|SelectInt (Math|Integer|SelectInt 0 (Utilities|Array|LastIndex (Variables|Default|GetOwnedGuns)) EnableIndexLoop) (LocalVariables|GetNextIndex) (> (LocalVariables|GetNextIndex) (Utilities|Array|LastIndex (Variables|Default|GetOwnedGuns)))))
      ;[1 1 1] Retrieve fluid gun from array
      (return (Utilities|Struct|BreakFluidGunProperties (Utilities|Array|Get(acopy) (Variables|Default|GetOwnedGuns) (LocalVariables|GetCurrentIndex))))
      (else
        (return "")))
    (else
      (return ""))))

(fn PreviousFluidGun
  (params (EnableIndexLoop :type Boolean))
  (if (Utilities|Array|IsNotEmpty (Variables|Default|GetOwnedGuns)) ; Check if array is empty.
    ;[1 1 1] Cache current fluid gun index and check if it is a valid index in the OwnedGuns array.
    (bind _output_get (LocalVariables|SetCurrentIndex (Class|FGFluidGunComponent|GetCurrentFluidGunIndex)))
    (if (Utilities|Array|IsValidIndex (Variables|Default|GetOwnedGuns) _output_get)
      (LocalVariables|SetNextIndex (- (LocalVariables|GetCurrentIndex) 1))
      (LocalVariables|SetCurrentIndex (Math|Integer|SelectInt (Math|Integer|SelectInt (Utilities|Array|LastIndex (Variables|Default|GetOwnedGuns)) 0 EnableIndexLoop) (LocalVariables|GetNextIndex) (< (LocalVariables|GetNextIndex) 0)))
      ;[1 1 1] Retrieve fluid gun from array
      (return (Utilities|Struct|BreakFluidGunProperties (Utilities|Array|Get(acopy) (Variables|Default|GetOwnedGuns) (LocalVariables|GetCurrentIndex))))
      (else
        (return "")))
    (else
      (return ""))))

(fn SetMappingContext
  (Input|AddMappingContext (PlayerController|LocalPlayerSubsystems|GetEnhancedInputLocalPlayerSubsystem (Game|GetPlayerController 0)) "/Game/Inputs/IMC_FluidGunComponent.IMC_FluidGunComponent" 0 "(bIgnoreAllPressedKeysUntilRelease=True,bForceImmediately=False,bNotifyUserSettings=False)")
  (return))

(fn RefillTank
  (params (FluidType :type Gameplay%20Tag%20Structure))
  (Variables|Default|GetCurrentGun
    (:then
      ;[1 1 1] Check if fluid in current tank is of the same type as fluid type in source.
      (if (GameplayTags|MatchesTag (Utilities|Struct|BreakTankProperties (Variables|/Script/FluidGuns.FG_FluidGun|GetTank (Variables|Default|GetCurrentGun))) FluidType true)
        (Class|FGFluidGun|RefillTank (Variables|Default|GetCurrentGun))
        (return true)
        (else
          (return false))))
    (:else)))