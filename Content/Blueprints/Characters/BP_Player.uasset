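; BP_Player is the player character Blueprint, which carries a fluid gun component for picked-up guns and tanks.
; On BeginPlay it registers itself as that component's owning character.
; AddGun and AddTank call their parent versions, then pass the data assets to the component; a new gun is also drawn immediately by its gameplay tag.
; Getters expose the component and character tags, while RefillTank always returns false.
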(event EventAddTank
  (params (TankDA :type FG%20PDA%20Tank%20Object%20Reference))
  (|CallParentFunction TankDA)
  (Class|FGFluidGunComponent|AddTank (Variables|Default|GetBP_FluidGunComponent) TankDA))

(event EventBeginPlay
  (|CallParentFunction)
  (Variables|/Game/Blueprints/Components/BP_FluidGunComponent.BP_FluidGunComponent_C|SetPlayerCharacter (Variables|Default|GetBP_FluidGunComponent) self))

(event EventAddGun
  (params (FluidGunDA :type FG%20PDA%20Fluid%20Gun%20Object%20Reference))
  (|CallParentFunction FluidGunDA)
  (Class|FGFluidGunComponent|AddFluidGun (Variables|Default|GetBP_FluidGunComponent) FluidGunDA)
  (Class|FGFluidGunComponent|DrawFluidGun (Variables|Default|GetBP_FluidGunComponent) (Variables|/Script/FluidGuns.FG_PDA_Item|GetItemGameplayTag FluidGunDA)) ; Draw picked-up fluid gun.
)

(fn ConstructionScript)

(fn RefillTank
  (params (FluidType :type Gameplay%20Tag%20Structure))
  (return false))

(fn RetrieveGameplayTagContainer
  (return (Variables|Default|GetCharacterGameplayTag)))

(fn ReturnFluidGunComponent
  (return (Variables|Default|GetBP_FluidGunComponent)))